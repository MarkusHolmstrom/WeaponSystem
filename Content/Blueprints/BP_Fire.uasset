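; BP_Fire is a fire actor that spreads by spawning copies of itself onto nearby actors tagged Burnable.
; One second after BeginPlay, Propagate increments a counter that selects an offset, then line-traces downward there with debug drawing.
; Burnable hits spawn another BP_Fire at that offset, while Glowable hits only print a message.
; Propagate re-runs after a delay only if the counter exceeds four; a surface-type switch is left unconnected.
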(event `self.ReceiveBeginPlay`
  (`KismetSystemLibrary.Delay` 1.0)
  (`self.Propagate`))

(event `self.ReceiveTick`
  (params (DeltaSeconds :type "Float (single-precision)")))

(event `Propagate`
  (bind _propagatedcount (`self.PropagatedCount`))
  (bind _returnvalue (select `int` _propagatedcount :`0` (1.0 0.0 0.0) :`1` (1.0 1.0 0.0) :`2` (-1.0 0.0 0.0) :`3` (-1.0 -1.0 0.0) :!type "Vector Structure"))
  (bind _returnvalue_2 (+ (* _returnvalue 90.0) (`self.K2_GetActorLocation`)))
  (`/Engine/EditorBlueprintResources/StandardMacros.IncrementInt` _propagatedcount
    (:`  `
      (`|ExecutionSequence`
        (:`then_0`
          (`KismetSystemLibrary.PrintString` (`KismetStringLibrary.Conv_VectorToString` _returnvalue) true false (struct :`G` 0.66 :`B` 1.0 :`A` 1.0) 1.0)
          (bind (_outhit _returnvalue_3) (`KismetSystemLibrary.LineTraceSingle` :`Start` (+ _returnvalue_2 (0.0 0.0 100.0)) :`End` (+ _returnvalue_2 (0.0 0.0 -100.0)) :`TraceChannel` "TraceTypeQuery1" :`DrawDebugType` "ForDuration"))
          (bind (_bblockinghit _binitialoverlap _time _distance _location _impactpoint _normal _impactnormal _physmat _hitactor) (`GameplayStatics.BreakHitResult` _outhit))
          (`KismetSystemLibrary.PrintString` (`KismetSystemLibrary.GetDisplayName` _hitactor))
          (if _returnvalue_3
            (if (`self.ActorHasTag` _hitactor "Burnable")
              (`|SpawnActorFromClass` "BP_Fire_C" (`KismetMathLibrary.MakeTransform` _returnvalue_2) "Undefined" "OverrideRootScale" null null)
              (elif (`self.ActorHasTag` _hitactor "Glowable")
                (`KismetSystemLibrary.PrintString` "nu gloder det")))))
        (:`then_1`
          (`KismetSystemLibrary.Delay` 2.0)
          (if (> _propagatedcount 4)
            (`self.Propagate`)))))))

(fn `UserConstructionScript`)
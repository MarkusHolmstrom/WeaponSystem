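; BP_Fire is a fire actor that spreads by spawning copies of itself onto nearby burnable or glowable surfaces.
; One second after BeginPlay, a randomized, incremented counter selects one of four fixed horizontal offsets for a vertical debug-drawn line trace.
; A tagged hit that casts to FireInteractableActor receives Interact and gets a new BP_Fire at that offset.
; The delayed repeat needs a counter above 12, which the starting range never reaches.
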(event `self.ReceiveBeginPlay`
  (`KismetSystemLibrary.Delay` 1.0)
  (set `self.PropagatedCount` (`KismetMathLibrary.RandomIntegerInRange` -1 3))
  (`self.Propagate`))

(event `Propagate`
  (bind _propagatedcount (`self.PropagatedCount`))
  (bind _returnvalue (+ (* (select `int` _propagatedcount :`0` (1.0 0.0 0.0) :`1` (1.0 1.0 0.0) :`2` (-1.0 0.0 0.0) :`3` (-1.0 -1.0 0.0) :!type "Vector Structure") 60.0) (`self.K2_GetActorLocation`)))
  (bind _result (`/Engine/EditorBlueprintResources/StandardMacros.IncrementInt` _propagatedcount)
    (:`  `
      (`|ExecutionSequence`
        (:`then_0`
          (bind (_outhit _returnvalue_2) (`KismetSystemLibrary.LineTraceSingle` :`Start` (+ _returnvalue (0.0 0.0 100.0)) :`End` (+ _returnvalue (0.0 0.0 -100.0)) :`TraceChannel` "TraceTypeQuery1" :`DrawDebugType` "ForDuration"))
          (if _returnvalue_2
            (bind (_bblockinghit _binitialoverlap _time _distance _location _impactpoint _normal _impactnormal _physmat _hitactor) (`GameplayStatics.BreakHitResult` _outhit))
            (if (`self.ActorHasTag` _hitactor "Burnable")
              (bind _asfire_interactable_actor (cast `FireInteractableActor` _hitactor :!label _label))
              (`FireInteractableActor.Interact` _asfire_interactable_actor)
              (`|SpawnActorFromClass` "BP_Fire_C" (`KismetMathLibrary.MakeTransform` _returnvalue) "Undefined" "OverrideRootScale" null null)
              (elif (`self.ActorHasTag` _hitactor "Glowable")
                (goto _label)))))
        (:`then_1`
          (`KismetSystemLibrary.Delay` 1.0)
          (if (> _propagatedcount 12)
            (set `self.PropagatedCount` 0)
            (`self.Propagate`)))))))

(fn `UserConstructionScript`)